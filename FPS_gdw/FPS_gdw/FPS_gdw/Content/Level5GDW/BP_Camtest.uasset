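; BP_Camtest is a test actor that catches the first-person character when its PawnSensing component sees them.
; On sight it disables that character's input, sets a CamCaught flag and eases its own rotation toward the player with RInterpTo and a look-at rotation.
; The rotation takes one interpolation step per sighting event rather than running on Tick.
; A disabled, unconnected branch would have enabled physics on meshes and the capsule after a short delay.
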(event `self.PawnSensing.OnSeePawn`
  (params (Pawn :type "Pawn Object Reference"))
  (bind _asbp_first_person_character (cast `/Game/FirstPerson/Blueprints/BP_FirstPersonCharacter` Pawn))
  (`self.DisableInput` _asbp_first_person_character (`GameplayStatics.GetPlayerController` 0))
  (set `self.CamCaught?` true)
  (bind _asbp_first_person_character_2 (cast `/Game/FirstPerson/Blueprints/BP_FirstPersonCharacter` (`GameplayStatics.GetPlayerCharacter` 0)))
  (`self.K2_SetActorRotation` (`KismetMathLibrary.RInterpTo` (`self.K2_GetActorRotation`) (`KismetMathLibrary.FindLookAtRotation` (`self.K2_GetActorLocation`) (`CharacterMovementComponent.GetLastUpdateLocation` (`Character.CharacterMovement` _asbp_first_person_character_2))) (`GameplayStatics.GetWorldDeltaSeconds`) 10.0)))

(fn `UserConstructionScript`)