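; BP_CAMZOOMOUTSMALLER is a pawn-sensing camera actor that watches for the first-person player and handles a death-and-respawn sequence.
; On seeing the player, it sets CamZoomCa and smoothly rotates toward the character's last updated location.
; Separately, Tick polls the character's DeathUI flag, then after short delays shows an animated DeadCamera_WD widget and opens the CamLevelRespawn level.
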(event `self.ReceiveTick`
  (params (DeltaSeconds :type "Float (single-precision)"))
  ;[1 1 1] Shows Widget
  (bind _outactors (`GameplayStatics.GetAllActorsOfClass` "/Game/FirstPerson/Blueprints/BP_FirstPersonCharacter.BP_FirstPersonCharacter_C"))
  (if (`/Game/FirstPerson/Blueprints/BP_FirstPersonCharacter.DeathUI?` (`|GetArrayItem` _outactors))
    (`KismetSystemLibrary.Delay` 0.8)
    (bind _returnvalue (`|CreateWidget` "/Game/DeadWidgets/DeadCamera_WD.DeadCamera_WD_C"))
    (`UserWidget.AddToViewport` _returnvalue 0)
    (`UserWidget.PlayAnimation` _returnvalue (`/Game/DeadWidgets/DeadCamera_WD.CamAnim` _returnvalue) 0.0 1 "Forward" 1.0 false)
    (`KismetSystemLibrary.Delay` 1.5)
    (`GameplayStatics.OpenLevel` (`self.CamLevelRespawn`))))

(event `self.PawnSensing.OnSeePawn`
  (params (Pawn :type "Pawn Object Reference"))
  ;[1 1 1] see player and looks at them
  (cast `/Game/FirstPerson/Blueprints/BP_FirstPersonCharacter` Pawn)
  (set `self.CamZoomCa?` true)
  (bind _asbp_first_person_character (cast `/Game/FirstPerson/Blueprints/BP_FirstPersonCharacter` (`GameplayStatics.GetPlayerCharacter` 0)))
  (`self.K2_SetActorRotation` (`KismetMathLibrary.RInterpTo` (`self.K2_GetActorRotation`) (`KismetMathLibrary.FindLookAtRotation` (`self.K2_GetActorLocation`) (`CharacterMovementComponent.GetLastUpdateLocation` (`Character.CharacterMovement` _asbp_first_person_character))) (`GameplayStatics.GetWorldDeltaSeconds`) 10.0)))

(fn `UserConstructionScript`)