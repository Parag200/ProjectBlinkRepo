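; BP_CAMZOOMOUT is a sensing actor, apparently a camera, that detects the first-person player and turns toward them.
; When PawnSensing sees a BP_FirstPersonCharacter, it sets the CamZoomCaught flag, which nothing in this graph reads or clears.
; It then interpolates its whole-actor rotation toward player 0's last movement update location.
; The rotation advances only on sensing events, with no Tick or timeline.
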(event `self.PawnSensing.OnSeePawn`
  (params (Pawn :type "Pawn Object Reference"))
  (cast `/Game/FirstPerson/Blueprints/BP_FirstPersonCharacter` Pawn)
  (set `self.CamZoomCaught?` true)
  (bind _asbp_first_person_character (cast `/Game/FirstPerson/Blueprints/BP_FirstPersonCharacter` (`GameplayStatics.GetPlayerCharacter` 0)))
  (`self.K2_SetActorRotation` (`KismetMathLibrary.RInterpTo` (`self.K2_GetActorRotation`) (`KismetMathLibrary.FindLookAtRotation` (`self.K2_GetActorLocation`) (`CharacterMovementComponent.GetLastUpdateLocation` (`Character.CharacterMovement` _asbp_first_person_character))) (`GameplayStatics.GetWorldDeltaSeconds`) 10.0)))

(fn `UserConstructionScript`)