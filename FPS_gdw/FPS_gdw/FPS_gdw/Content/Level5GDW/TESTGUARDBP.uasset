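; TESTGUARDBP is a test guard enemy that loops through four waypoints using AI MoveTo and can shoot at the first-person player.
; Pawn sensing turns it toward a seen player and, if that player's LookingAtGuard is set, fires one GuardBullet from an arrow component after a short delay.
; Tick slows the guard's time dilation once the player's HasSlowed is true, with no reset here.
; Hits from pistol-tagged actors destroy it.
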(event `self.ReceiveTick`
  (params (DeltaSeconds :type "Float (single-precision)"))
  ;[1 1 1] Goes into slo mo
  (bind _outactors (`GameplayStatics.GetAllActorsOfClass` "/Game/FirstPerson/Blueprints/BP_FirstPersonCharacter.BP_FirstPersonCharacter_C"))
  (if (`/Game/FirstPerson/Blueprints/BP_FirstPersonCharacter.HasSlowed?` (`|GetArrayItem` _outactors))
    (set `self.CustomTimeDilation` 0.2)))

(event `self.ReceiveBeginPlay`
  ;[1 1 1] Follows Way Point
  (`|AIMoveTo` self (`self.Way1`) null :!label _label
    (:`OnSuccess`
      (`|AIMoveTo` self (`self.Way2`) null
        (:`OnSuccess`
          (`|AIMoveTo` self (`self.Way3`) null
            (:`OnSuccess`
              (`|AIMoveTo` self (`self.Way4`) null
                (:`OnSuccess`
                  (goto _label))))))))))

(event `self.PawnSensing.OnSeePawn`
  (params (Pawn :type "Pawn Object Reference"))
  ;[1 1 1] When sees player it will turn to face aplayer
  (cast `/Game/FirstPerson/Blueprints/BP_FirstPersonCharacter` Pawn)
  (set `self.PlayerCaughtGuard?` true)
  (bind _asbp_first_person_character (cast `/Game/FirstPerson/Blueprints/BP_FirstPersonCharacter` Pawn))
  (`self.K2_SetActorRotation` (`KismetMathLibrary.RInterpTo` (`self.K2_GetActorRotation`) (`KismetMathLibrary.FindLookAtRotation` (`self.K2_GetActorLocation`) (`CharacterMovementComponent.GetLastUpdateLocation` (`Character.CharacterMovement` _asbp_first_person_character))) (`GameplayStatics.GetWorldDeltaSeconds`) 5.5))
  (bind _outactors (`GameplayStatics.GetAllActorsOfClass` "/Game/FirstPerson/Blueprints/BP_FirstPersonCharacter.BP_FirstPersonCharacter_C"))
  (if (`/Game/FirstPerson/Blueprints/BP_FirstPersonCharacter.LookingAtGuard?` (`|GetArrayItem` _outactors))
    (`KismetSystemLibrary.Delay` 0.7)
    (`/Engine/EditorBlueprintResources/StandardMacros.DoOnce` false
      (:`Completed`
        (`|SpawnActorFromClass` "/Game/Level5GDW/GuardBullet.GuardBullet_C" (`SceneComponent.K2_GetComponentToWorld` (`self.Arrow1`)) "Undefined" "MultiplyWithRoot" null null)
        (set `self.ShotBullet?` true)))))

(event `self.CapsuleComponent.OnComponentHit`
  (params (HitComponent :type "PrimitiveComponent Object Reference") (OtherActor :type "Actor Object Reference") (OtherComp :type "PrimitiveComponent Object Reference") (NormalImpulse :type "Vector Structure") (Hit :type "HitResult Structure (by ref)"))
  ;[1 1 1] dies if hit with pistol
  (if (`self.ActorHasTag` OtherActor "pistol")
    (`self.K2_DestroyActor`)))

(fn `UserConstructionScript`)