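; BP_Guard is a patrolling enemy that kills the first-person player on sight and respawns them.
; Tick moves only the mesh along a local spline with height and yaw offsets, resetting at the end when looping is enabled.
; Pawn sensing destroys the player, plays a death widget animation, then spawns and possesses a new character at RespawnLocation.
; The Hit event destroys the guard.
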(event `self.ReceiveTick`
  (params (DeltaSeconds :type "Float (single-precision)"))
  (bind _returnvalue (`SplineComponent.GetTransformAtDistanceAlongSpline` (`self.Spline`) (`self.Distance Along Spline`) "Local" false))
  (set `self.Distance Along Spline` (+ (* DeltaSeconds (`self.Spline Speed`)) (`self.Distance Along Spline`)))
  (`SceneComponent.K2_SetRelativeTransform` (`self.Mesh`) (`KismetMathLibrary.MakeTransform` (`KismetMathLibrary.MakeVector` (.x (.location _returnvalue)) (.y (.location _returnvalue)) (+ (.z (.location _returnvalue)) -89.0)) (`KismetMathLibrary.MakeRotator` (.roll (.rotation _returnvalue)) (.pitch (.rotation _returnvalue)) (+ (.yaw (.rotation _returnvalue)) -90.0))) false false)
  (if (`self.isLoop?`)
    (if (> (`self.Distance Along Spline`) (`SplineComponent.GetSplineLength` (`self.Spline`)))
      (set `self.Distance Along Spline` 0.0))))

(event `self.ReceiveHit`
  (params (MyComp :type "PrimitiveComponent Object Reference") (Other :type "Actor Object Reference") (OtherComp :type "PrimitiveComponent Object Reference") (bSelfMoved :type Boolean) (HitLocation :type "Vector Structure") (HitNormal :type "Vector Structure") (NormalImpulse :type "Vector Structure") (Hit :type "HitResult Structure (by ref)"))
  (`self.K2_DestroyActor`))

(event `self.PawnSensing.OnSeePawn`
  (params (Pawn :type "Pawn Object Reference"))
  (bind _asbp_first_person_character (cast `/Game/FirstPerson/Blueprints/BP_FirstPersonCharacter` Pawn))
  (`KismetSystemLibrary.PrintString` "Hello")
  (`self.K2_DestroyActor` _asbp_first_person_character)
  (bind _returnvalue (`|CreateWidget` "/Game/DeadWidgets/DeadGuard_WD.DeadGuard_WD_C"))
  (`UserWidget.AddToViewport` _returnvalue 0)
  (`UserWidget.PlayAnimation` _returnvalue (`/Game/DeadWidgets/DeadGuard_WD.GuardAnim` _returnvalue) 0.0 1 "Forward" 1.0 false)
  (`GameplayStatics.GetAllActorsOfClass` "/Game/Level1GDW/Level1Assets/Triggers/BP_Respawn.BP_Respawn_C")
  (bind _returnvalue_2 (`|SpawnActorFromClass` "/Game/FirstPerson/Blueprints/BP_FirstPersonCharacter.BP_FirstPersonCharacter_C" (`KismetMathLibrary.Conv_VectorToTransform` (`self.RespawnLocation`)) "Undefined" "MultiplyWithRoot" null null))
  (`Controller.Possess` (`GameplayStatics.GetPlayerController` 0) _returnvalue_2))

(fn `UserConstructionScript`)