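; Enemy guard that carries a key card and ends the player's run on sight.
; It loops through four waypoints with chained AI Move To calls, repeating only while each move succeeds.
; When pawn sensing sees the first-person character, it destroys that character, plays a death widget animation and opens a named level after a short delay.
; A hit from a pistol-tagged actor destroys the guard and spawns a key card at a set location.
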(event `self.ReceiveBeginPlay`
  ;[1 1 1] Follows Way Point
  (`|AIMoveTo` self (`self.Way1`) null :!label _label
    (:`OnSuccess`
      (`|AIMoveTo` self (`self.Way2`) null
        (:`OnSuccess`
          (`|AIMoveTo` self (`self.Way3`) null
            (:`OnSuccess`
              (`|AIMoveTo` self (`self.Way4`) null
                (:`OnSuccess`
                  (goto _label))))))))))

(event `self.PawnSensing.OnSeePawn`
  (params (Pawn :type "Pawn Object Reference"))
  ;[1 1 1] When sees player
  (bind _asbp_first_person_character (cast `/Game/FirstPerson/Blueprints/BP_FirstPersonCharacter` Pawn))
  (`self.K2_DestroyActor` _asbp_first_person_character)
  (bind _returnvalue (`|CreateWidget` "/Game/DeadWidgets/DeadGuard_WD.DeadGuard_WD_C"))
  (`UserWidget.AddToViewport` _returnvalue 0)
  (`UserWidget.PlayAnimation` _returnvalue (`/Game/DeadWidgets/DeadGuard_WD.GuardAnim` _returnvalue) 0.0 1 "Forward" 1.0 false)
  (`KismetSystemLibrary.Delay` 0.4)
  (`GameplayStatics.OpenLevel` (`self.NameLevel`)))

(event `self.CapsuleComponent.OnComponentHit`
  (params (HitComponent :type "PrimitiveComponent Object Reference") (OtherActor :type "Actor Object Reference") (OtherComp :type "PrimitiveComponent Object Reference") (NormalImpulse :type "Vector Structure") (Hit :type "HitResult Structure (by ref)"))
  ;[1 1 1] dies if hit with pistol
  (if (`self.ActorHasTag` OtherActor "pistol")
    (`self.K2_DestroyActor`)
    (`|SpawnActorFromClass` "/Game/Level1GDW/Level1Assets/Enemy/BP_KeyCard.BP_KeyCard_C" (`KismetMathLibrary.MakeTransform` (`self.KeyCardSpawn`)) "Undefined" "MultiplyWithRoot" null null)))

(fn `UserConstructionScript`)