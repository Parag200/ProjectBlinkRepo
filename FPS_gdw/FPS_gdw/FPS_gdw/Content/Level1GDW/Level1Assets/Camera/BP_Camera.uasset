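; BP_Camera is a security-camera hazard that fails the player on sight and restarts play.
; Its PawnSensing component detects pawns, and a BP_FirstPersonCharacter that is seen gets destroyed.
; It then shows the DeadCamera_WD widget with its animation and, after a short delay, opens the level named by CamLevelRespawn.
; On BeginPlay it also makes its Cube component visible.
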(event `self.ReceiveBeginPlay`
  (`SceneComponent.SetVisibility` (`self.Cube`) true false))

(event `self.PawnSensing.OnSeePawn`
  (params (Pawn :type "Pawn Object Reference"))
  (bind _asbp_first_person_character (cast `/Game/FirstPerson/Blueprints/BP_FirstPersonCharacter` Pawn))
  (`self.K2_DestroyActor` _asbp_first_person_character)
  (bind _returnvalue (`|CreateWidget` "/Game/DeadWidgets/DeadCamera_WD.DeadCamera_WD_C"))
  (`UserWidget.AddToViewport` _returnvalue 0)
  (`UserWidget.PlayAnimation` _returnvalue (`/Game/DeadWidgets/DeadCamera_WD.CamAnim` _returnvalue) 0.0 1 "Forward" 1.0 false)
  (`KismetSystemLibrary.Delay` 1.0)
  (`GameplayStatics.OpenLevel` (`self.CamLevelRespawn`)))

(fn `UserConstructionScript`)