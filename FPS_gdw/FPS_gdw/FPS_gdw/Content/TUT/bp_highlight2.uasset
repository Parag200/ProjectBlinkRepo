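; Tutorial trigger actor that plays a narrated sequence once when a component tagged "player" enters its box.
; It disables the player character's input, then plays three 2D sounds (after teleport, turn green, reload) separated by fixed delays.
; Input is re-enabled after the last delay, with DoOnce nodes guarding each step so it cannot replay.
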(event `self.Box.OnComponentBeginOverlap`
  (params (OverlappedComponent :type "PrimitiveComponent Object Reference") (OtherActor :type "Actor Object Reference") (OtherComp :type "PrimitiveComponent Object Reference") (OtherBodyIndex :type Integer) (bFromSweep :type Boolean) (SweepResult :type "HitResult Structure (by ref)"))
  (if (`ActorComponent.ComponentHasTag` OtherComp "player")
    (`/Engine/EditorBlueprintResources/StandardMacros.DoOnce` false
      (:`Completed`
        (`self.DisableInput` (`GameplayStatics.GetPlayerCharacter` 0) (`GameplayStatics.GetPlayerController` 0))
        (`/Engine/EditorBlueprintResources/StandardMacros.DoOnce` false
          (:`Completed`
            (`GameplayStatics.PlaySound2D` "/Game/TUT/voices/afterTP.afterTP" 1.0 1.0 0.0 null null)
            (`KismetSystemLibrary.Delay` 4.0)
            (`/Engine/EditorBlueprintResources/StandardMacros.DoOnce` false
              (:`Completed`
                (`GameplayStatics.PlaySound2D` "/Game/TUT/voices/turn_green.turn_green" 1.0 1.0 0.0 null null)
                (`KismetSystemLibrary.Delay` 4.0)
                (`/Engine/EditorBlueprintResources/StandardMacros.DoOnce` false
                  (:`Completed`
                    (`GameplayStatics.PlaySound2D` "/Game/TUT/voices/Reload.Reload" 1.0 1.0 0.0 null null)
                    (`KismetSystemLibrary.Delay` 3.0)
                    (`/Engine/EditorBlueprintResources/StandardMacros.DoOnce` false
                      (:`Completed`
                        (`self.EnableInput` (`GameplayStatics.GetPlayerCharacter` 0) (`GameplayStatics.GetPlayerController` 0))))))))))))))

(fn `UserConstructionScript`)