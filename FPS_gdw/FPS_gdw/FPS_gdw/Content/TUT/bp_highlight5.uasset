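; Tutorial trigger actor that briefly freezes the player and plays the "Last" sound when the player enters its box.
; The box overlap checks the other component for the "player" tag, disables input on player character 0, plays the 2D sound and re-enables input after a two-second delay.
; DoOnce gates make the whole sequence fire only once, with no reset.
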(event `self.Box.OnComponentBeginOverlap`
  (params (OverlappedComponent :type "PrimitiveComponent Object Reference") (OtherActor :type "Actor Object Reference") (OtherComp :type "PrimitiveComponent Object Reference") (OtherBodyIndex :type Integer) (bFromSweep :type Boolean) (SweepResult :type "HitResult Structure (by ref)"))
  (bind _returnvalue (`GameplayStatics.GetPlayerController` 0))
  (bind _returnvalue_2 (`GameplayStatics.GetPlayerCharacter` 0))
  (if (`ActorComponent.ComponentHasTag` OtherComp "player")
    (`/Engine/EditorBlueprintResources/StandardMacros.DoOnce` false
      (:`Completed`
        (`self.DisableInput` _returnvalue_2 _returnvalue)
        (`/Engine/EditorBlueprintResources/StandardMacros.DoOnce` false
          (:`Completed`
            (`GameplayStatics.PlaySound2D` "/Game/TUT/voices/last.last" 1.0 1.0 0.0 null null)
            (`KismetSystemLibrary.Delay` 2.0)
            (`/Engine/EditorBlueprintResources/StandardMacros.DoOnce` false
              (:`Completed`
                (`self.EnableInput` _returnvalue_2 _returnvalue)))))))))

(fn `UserConstructionScript`)