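; Guard enemy that patrols four waypoints in a looping AIMoveTo chain and drops a keycard when destroyed by a pistol-tagged hit.
; On seeing the player it sets caught state and turns toward them; player flags gate a delayed death widget and level load.
; Tick polls the first-person character through GetAllActorsOfClass to apply slow motion to the guard or halt its movement.
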(event `self.ReceiveTick`
  (params (DeltaSeconds :type "Float (single-precision)"))
  ;[1 1 1] Goes into slo mo
  (`|ExecutionSequence`
    (:`then_0`
      (bind _outactors (`GameplayStatics.GetAllActorsOfClass` "/Game/FirstPerson/Blueprints/BP_FirstPersonCharacter.BP_FirstPersonCharacter_C"))
      (if (`/Game/FirstPerson/Blueprints/BP_FirstPersonCharacter.HasSlowed?` (`|GetArrayItem` _outactors))
        (set `self.CustomTimeDilation` 0.2)))
    (:`then_1`
      (bind _outactors_2 (`GameplayStatics.GetAllActorsOfClass` "/Game/FirstPerson/Blueprints/BP_FirstPersonCharacter.BP_FirstPersonCharacter_C"))
      (if (`/Game/FirstPerson/Blueprints/BP_FirstPersonCharacter.GuardStopMoving?` (`|GetArrayItem` _outactors_2))
        (`MovementComponent.StopMovementImmediately` (`self.CharacterMovement`))))))

(event `self.ReceiveBeginPlay`
  ;[1 1 1] Follows Way Point
  (`|AIMoveTo` self (`self.Way1`) null :!label _label
    (:`OnSuccess`
      (`|AIMoveTo` self (`self.Way2`) null
        (:`OnSuccess`
          (`|AIMoveTo` self (`self.Way3`) null
            (:`OnSuccess`
              (`|AIMoveTo` self (`self.Way4`) null
                (:`OnSuccess`
                  (goto _label))))))))))

(event `self.PawnSensing.OnSeePawn`
  (params (Pawn :type "Pawn Object Reference"))
  ;[1 1 1] When sees player it will turn to face aplayer
  (cast `/Game/FirstPerson/Blueprints/BP_FirstPersonCharacter` Pawn)
  (set `self.PlayerCaught?` true)
  (bind _asbp_first_person_character (cast `/Game/FirstPerson/Blueprints/BP_FirstPersonCharacter` Pawn))
  (`self.K2_SetActorRotation` (`KismetMathLibrary.RInterpTo` (`self.K2_GetActorRotation`) (`KismetMathLibrary.FindLookAtRotation` (`self.K2_GetActorLocation`) (`CharacterMovementComponent.GetLastUpdateLocation` (`Character.CharacterMovement` _asbp_first_person_character))) (`GameplayStatics.GetWorldDeltaSeconds`) 5.5))
  (bind _outactors (`GameplayStatics.GetAllActorsOfClass` "/Game/FirstPerson/Blueprints/BP_FirstPersonCharacter.BP_FirstPersonCharacter_C"))
  (if (`/Game/FirstPerson/Blueprints/BP_FirstPersonCharacter.LookingAtGuard?` (`|GetArrayItem` _outactors))
    (`KismetSystemLibrary.Delay` 0.8)
    (set `self.PlayerSim?` true)
    (bind _outactors_2 (`GameplayStatics.GetAllActorsOfClass` "/Game/FirstPerson/Blueprints/BP_FirstPersonCharacter.BP_FirstPersonCharacter_C"))
    (if (`/Game/FirstPerson/Blueprints/BP_FirstPersonCharacter.DeathUIGuard?` (`|GetArrayItem` _outactors_2))
      (`KismetSystemLibrary.Delay` 1.4)
      (bind _returnvalue (`|CreateWidget` "/Game/DeadWidgets/DeadGuard_WD.DeadGuard_WD_C"))
      (`UserWidget.AddToViewport` _returnvalue 0)
      (`UserWidget.PlayAnimation` _returnvalue (`/Game/DeadWidgets/DeadGuard_WD.GuardAnim` _returnvalue) 0.0 1 "Forward" 1.0 false)
      (`KismetSystemLibrary.Delay` 1.6)
      (`GameplayStatics.OpenLevel` (`self.LevelName`)))))

(event `self.CapsuleComponent.OnComponentHit`
  (params (HitComponent :type "PrimitiveComponent Object Reference") (OtherActor :type "Actor Object Reference") (OtherComp :type "PrimitiveComponent Object Reference") (NormalImpulse :type "Vector Structure") (Hit :type "HitResult Structure (by ref)"))
  ;[1 1 1] dies if hit with pistol
  (if (`self.ActorHasTag` OtherActor "pistol")
    (`self.K2_DestroyActor`)
    (`|SpawnActorFromClass` "/Game/Level4GDW/BP_KeyCard.BP_KeyCard_C" (`KismetMathLibrary.MakeTransform` (`self.KeyCardSpawn`)) "Undefined" "MultiplyWithRoot" null null)))

(fn `UserConstructionScript`)