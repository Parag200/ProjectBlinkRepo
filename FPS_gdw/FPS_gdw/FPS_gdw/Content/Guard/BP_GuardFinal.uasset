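; Guard enemy that patrols a loop of four waypoints with AI MoveTo and reacts to seeing the player.
; Pawn sensing flags the player as caught, turns toward them and, if they are looking back, plays an aim animation and sets PlayerSimulate.
; Pistol-tagged overlaps play a hit sound and death animation, then swap the guard for a dart actor.
; Tick polls player flags to slow the guard's time, stop movement or open a level.
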(event `self.ReceiveTick`
  (params (DeltaSeconds :type "Float (single-precision)"))
  ;[1 1 1] Goes into slo mo
  (`|ExecutionSequence`
    (:`then_0`
      (bind _outactors (`GameplayStatics.GetAllActorsOfClass` "/Game/FirstPerson/Blueprints/BP_FirstPersonCharacter.BP_FirstPersonCharacter_C"))
      (if (`/Game/FirstPerson/Blueprints/BP_FirstPersonCharacter.HasSlowed?` (`|GetArrayItem` _outactors))
        (set `self.CustomTimeDilation` 0.2)))
    (:`then_1`
      (bind _outactors_2 (`GameplayStatics.GetAllActorsOfClass` "/Game/FirstPerson/Blueprints/BP_FirstPersonCharacter.BP_FirstPersonCharacter_C"))
      (if (`/Game/FirstPerson/Blueprints/BP_FirstPersonCharacter.GuardStopMoving?` (`|GetArrayItem` _outactors_2))
        (`MovementComponent.StopMovementImmediately` (`self.CharacterMovement`))))
    (:`then_2`
      (bind _outactors_3 (`GameplayStatics.GetAllActorsOfClass` "/Game/FirstPerson/Blueprints/BP_FirstPersonCharacter.BP_FirstPersonCharacter_C"))
      (if (`/Game/FirstPerson/Blueprints/BP_FirstPersonCharacter.OpenLevel?` (`|GetArrayItem` _outactors_3))
        (`GameplayStatics.OpenLevel` (`self.LevelName`))))))

(event `self.ReceiveBeginPlay`
  ;[1 1 1] Follows Way Point
  (`|AIMoveTo` self (`self.Way1`) null :!label _label
    (:`OnSuccess`
      (`|AIMoveTo` self (`self.Way2`) null
        (:`OnSuccess`
          (`|AIMoveTo` self (`self.Way3`) null
            (:`OnSuccess`
              (`|AIMoveTo` self (`self.Way4`) null
                (:`OnSuccess`
                  (goto _label))))))))))

(event `self.PawnSensing.OnSeePawn`
  (params (Pawn :type "Pawn Object Reference"))
  ;[1 1 1] When sees player it will turn to face aplayer
  (cast `/Game/FirstPerson/Blueprints/BP_FirstPersonCharacter` Pawn)
  (set `self.PlayerCaughtGuard?` true)
  (bind _asbp_first_person_character (cast `/Game/FirstPerson/Blueprints/BP_FirstPersonCharacter` Pawn))
  (`self.K2_SetActorRotation` (`KismetMathLibrary.RInterpTo` (`self.K2_GetActorRotation`) (`KismetMathLibrary.FindLookAtRotation` (`self.K2_GetActorLocation`) (`CharacterMovementComponent.GetLastUpdateLocation` (`Character.CharacterMovement` _asbp_first_person_character))) (`GameplayStatics.GetWorldDeltaSeconds`) 5.5))
  (bind _outactors (`GameplayStatics.GetAllActorsOfClass` "/Game/FirstPerson/Blueprints/BP_FirstPersonCharacter.BP_FirstPersonCharacter_C"))
  (if (`/Game/FirstPerson/Blueprints/BP_FirstPersonCharacter.LookingAtGuard?` (`|GetArrayItem` _outactors))
    (`/Engine/EditorBlueprintResources/StandardMacros.DoOnce` false
      (:`Completed`
        (`SkeletalMeshComponent.PlayAnimation` (`self.Mesh`) "/Game/Guard/Mixamo/Animations/Rifle_Down_To_Aim.Rifle_Down_To_Aim" false)
        (`/Engine/EditorBlueprintResources/StandardMacros.DoOnce` false
          (:`Completed`
            (set `self.PlayerSimulate?` true)))))))

(event `self.CapsuleComponent.OnComponentBeginOverlap`
  (params (OverlappedComponent :type "PrimitiveComponent Object Reference") (OtherActor :type "Actor Object Reference") (OtherComp :type "PrimitiveComponent Object Reference") (OtherBodyIndex :type Integer) (bFromSweep :type Boolean) (SweepResult :type "HitResult Structure (by ref)"))
  ;[1 1 1] dies if hit with pistol
  (`|ExecutionSequence`
    (:`then_0`
      (if (`self.ActorHasTag` OtherActor "pistol")
        (`GameplayStatics.PlaySoundAtLocation` "/Game/SoundsFX/Guard_hit_sound.Guard_hit_sound" (`self.K2_GetActorLocation` self) (struct) 1.0 1.0 0.0 null null null null :!label _label_2)
        (`MovementComponent.StopMovementImmediately` (`self.CharacterMovement`))
        (`/Engine/EditorBlueprintResources/StandardMacros.DoOnce` false
          (:`Completed`
            (`SkeletalMeshComponent.PlayAnimation` (`self.Mesh`) "/Game/Guard/Mixamo/Animations/Walking_To_Dying__1_.Walking_To_Dying__1_" false)
            (`KismetSystemLibrary.Delay` 3.0)
            (`self.K2_DestroyActor`)
            (`|SpawnActorFromClass` "/Game/Guns+Animations/TPDart/Dart/BP_DartStillActor.BP_DartStillActor_C" (`KismetMathLibrary.MakeTransform` (`self.K2_GetActorLocation`)) "Undefined" "MultiplyWithRoot" null null)))))
    (:`then_1`
      (if (`ActorComponent.ComponentHasTag` OtherComp "pistol")
        (goto _label_2)))))

(fn `UserConstructionScript`)