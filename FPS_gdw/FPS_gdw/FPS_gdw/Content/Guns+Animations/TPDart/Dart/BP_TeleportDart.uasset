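; BP_TeleportDart is a teleport dart projectile that records a teleport location where it hits the world.
; A Niagara effect activates on spawn while ProjectileMovement carries the dart.
; When the capsule overlaps an actor tagged WorldOBJ, the dart stops, flags itself as stopped, turns off the effect and plays a hit sound.
; It stores the dart component's world location in TPLocation, then destroys itself after a short delay.
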(event `self.ReceiveBeginPlay`
  (`ActorComponent.SetActive` (`self.Niagara`) true false))

(event `self.Capsule.OnComponentBeginOverlap`
  (params (OverlappedComponent :type "PrimitiveComponent Object Reference") (OtherActor :type "Actor Object Reference") (OtherComp :type "PrimitiveComponent Object Reference") (OtherBodyIndex :type Integer) (bFromSweep :type Boolean) (SweepResult :type "HitResult Structure (by ref)"))
  (if (`self.ActorHasTag` OtherActor "WorldOBJ")
    (`MovementComponent.StopMovementImmediately` (`self.ProjectileMovement`))
    (set `self.HasDartStopped?` true)
    (`ActorComponent.Deactivate` (`self.Niagara`))
    (`GameplayStatics.PlaySound2D` "/Game/Guns+Animations/TPDart/Dart/DartHitFX.DartHitFX" 1.0 1.0 0.0 null null)
    (set `self.TPLocation` (`SceneComponent.K2_GetComponentLocation` (`self.Dart`)))
    (`KismetSystemLibrary.Delay` 1.5)
    (`self.K2_DestroyActor`)))

(fn `UserConstructionScript`)